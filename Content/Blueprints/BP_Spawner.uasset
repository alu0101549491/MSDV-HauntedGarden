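; Spawner actor that keeps the level populated with BP_Ghost actors around the BP_Girl character.
; Each Tick it counts existing ghosts and, while below NumEnemies, spawns one with the configured lifetime range.
; GetSpawnTransform places it at a random yaw direction, a set Distance from the girl, with random facing and width/height scaling, provided she is valid.
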(event `self.ReceiveTick`
  (params (DeltaSeconds :type "Float (single-precision)"))
  ; Handle Spawn of Ghosts
  (bind _outactors (`GameplayStatics.GetAllActorsOfClass` "/Game/Ghost/BP_Ghost.BP_Ghost_C"))
  (if (< (`KismetArrayLibrary.Array_Length` _outactors) (`self.NumEnemies`))
    (bind _transform (`self.GetSpawnTransform`)
      (:`ExecOut`
        (`|SpawnActorFromClass` "/Game/Ghost/BP_Ghost.BP_Ghost_C" _transform "AdjustIfPossibleButAlwaysSpawn" "MultiplyWithRoot" null (`self.MinLifeTime`) (`self.MaxLifeTime`) null)))))

(fn `UserConstructionScript`)