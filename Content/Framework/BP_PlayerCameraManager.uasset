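; Player camera manager that keeps the view at the MainCameraSlot actor's location and turns it to follow the player pawn.
; BlueprintUpdateCamera runs its logic only for a BP_Girl target, taking FOV from her camera and returning MainCamera as the override flag.
; RecalculateRotation passes the look-at rotation through, but beyond PitchLimit it holds the last safe rotation, yaw included, and sets InCriticalPitch.
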(fn `BlueprintUpdateCamera`
  (params (CameraTarget :type "Actor Object Reference"))
  (returns (NewCameraLocation :type "Vector Structure") (NewCameraRotation :type "Rotator Structure") (NewCameraFOV :type "Float (single-precision)") (ReturnValue :type Boolean))
  (bind _returnvalue (`self.K2_GetActorLocation` (`self.MainCameraSlot`)))
  (bind _asbp_girl (cast `/Game/Framework/BP_Girl` CameraTarget))
  (bind _desiredview (`CameraComponent.GetCameraView` (`/Game/Framework/BP_Girl.Camera` _asbp_girl) 0.0))
  (bind _rotationout (`self.RecalculateRotation` (`KismetMathLibrary.FindLookAtRotation` _returnvalue (`self.K2_GetActorLocation` (`GameplayStatics.GetPlayerPawn` 0)))))
  (return _returnvalue _rotationout (`.FOV` (break `MinimalViewInfo` _desiredview)) (`self.bMainCamera`)))

(fn `RecalculateRotation`
  (params (RotationIn :type "Rotator Structure"))
  (returns (RotationOut :type "Rotator Structure"))
  (if (> (`KismetMathLibrary.Abs` (.pitch RotationIn)) (`self.PitchLimit`))
    (set `self.bInCriticalPitch` true)
    (return (`self.FrozenRotation`))
    (else
      ; Pitch en zona segura
      (set `self.bInCriticalPitch` false)
      (bind _output_get (set `self.FrozenRotation` RotationIn))
      (return _output_get))))

(fn `UserConstructionScript`)