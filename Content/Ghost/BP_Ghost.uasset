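; BP_Ghost is an AI pawn that starts disguised as a mushroom, can turn into a killing ghost, and destroys itself after a random lifetime.
; Pawn sensing writes any seen BP_Girl into the AI blackboard as the target to follow.
; On capsule hit, the girl gets a positive outcome outside killing mode, or takes damage as the ghost destroys itself.
; OnKillingModeChange swaps the mushroom mesh for the ghost shape.
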(event `self.ReceiveBeginPlay`
  (`SceneComponent.SetHiddenInGame` (`self.GhostShape`) true false)
  ; Handle Time spanwed
  (`KismetSystemLibrary.Delay` (`KismetMathLibrary.RandomFloatInRange` (`self.MinLifeTime`) (`self.MaxLifeTime`)))
  (`self.K2_DestroyActor`))

(event `self.PawnSensing.OnSeePawn`
  (params (Pawn :type "Pawn Object Reference"))
  ; Set BP_Girl as Target to follow
  (bind _asbp_girl (cast `/Game/Framework/BP_Girl` Pawn))
  (`BlackboardComponent.SetValueAsObject` (`AIBlueprintHelperLibrary.GetBlackboard` (`self.GetController`)) (`self.KeyGirl`) _asbp_girl))

(event `OnKillingModeChange`
  ; Switch from Mushroom to Ghost
  (`SceneComponent.SetHiddenInGame` (`self.Mesh`) true false)
  (`SceneComponent.SetHiddenInGame` (`self.GhostShape`) false false))

(event `self.CapsuleComponent.OnComponentHit`
  (params (HitComponent :type "PrimitiveComponent Object Reference") (OtherActor :type "Actor Object Reference") (OtherComp :type "PrimitiveComponent Object Reference") (NormalImpulse :type "Vector Structure") (Hit :type "HitResult Structure (by ref)"))
  ; Damage Handling
  (bind _asbp_girl (cast `/Game/Framework/BP_Girl` OtherActor))
  (if (not (`self.IsKilling`))
    (`/Game/Framework/BP_Girl.PositiveOutcome` _asbp_girl (`self.Gains`))
    (else
      (`GameplayStatics.ApplyDamage` _asbp_girl (`self.Damage`) null self)
      (`self.K2_DestroyActor`))))

(fn `UserConstructionScript`)